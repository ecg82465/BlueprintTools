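; BP_FaceToPlayerCamera is a component that turns the scene component it is attached to toward the player's camera.
; Each Tick, while FaceToCamera is true, it computes a look-at rotation from the attach parent to the camera manager of player 0.
; It interpolates the parent's world rotation to that target at MoveSpeed, so the parent rotates rather than the component itself.
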(event EventBeginPlay)

(event EventTick
  (params (DeltaSeconds :type Float%20%28single-precision%29))
  (bind _returnvalue (Transformation|GetAttachParent))
  (if (Variables|Default|GetFaceToCamera)
    (Transformation|SetWorldRotation _returnvalue (Math|Interpolation|RInterpTo (Transformation|GetWorldRotation _returnvalue) (Math|Rotator|FindLookatRotation (Transformation|GetWorldLocation _returnvalue) (Transformation|GetActorLocation (Game|GetPlayerCameraManager 0))) (Utilities|Time|GetWorldDeltaSeconds) (Variables|Default|GetMoveSpeed)) false false)))