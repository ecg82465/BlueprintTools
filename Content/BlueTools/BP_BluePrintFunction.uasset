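; BP_BluePrintFunction is a set of utility functions for aspect-aware textures and spline distance lookup.
; Two AdaptiveTexture functions put a file-loaded or supplied texture on a dynamic material, setting X/Y scalar parameters to keep its aspect ratio, longer side at 1.
; FindSplineDistance converts a world location to distance along a spline by linearly interpolating between point distances around the closest input key.
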(fn AdaptiveTextureFile
  (params (FilePath :type String) (InputPin :type Material%20Instance%20Dynamic%20Object%20Reference))
  (bind (_isvalid _width _height _returnvalue) (Class|BlueprintUtilityBPLibrary|LoadTexture2DfromFile FilePath))
  (bind _returnvalue_2 (Math|Conversions|ToFloat(Integer) _width))
  (bind _returnvalue_3 (Math|Conversions|ToFloat(Integer) _height))
  (if _isvalid
    (Rendering|Material|SetTextureParameterValue InputPin "Texture" _returnvalue)
    (if (> _width _height)
      (Rendering|Material|SetScalarParameterValue InputPin "Y" (/ _returnvalue_3 _returnvalue_2) :!class /Script/Engine.MaterialInstanceDynamic)
      (Rendering|Material|SetScalarParameterValue InputPin "X" 1.0 :!class /Script/Engine.MaterialInstanceDynamic)
      (else
        (Rendering|Material|SetScalarParameterValue InputPin "X" (/ _returnvalue_2 _returnvalue_3) :!class /Script/Engine.MaterialInstanceDynamic)
        (Rendering|Material|SetScalarParameterValue InputPin "Y" 1.0 :!class /Script/Engine.MaterialInstanceDynamic)))))

(fn FindSplineDistance
  (params (InputPin :type Spline%20Component%20Object%20Reference) (WorldLocation :type Vector%20%28by%20ref%29))
  (bind _returnvalue (Class|SplineComponent|FindInputKeyClosesttoWorldLocation InputPin WorldLocation))
  (bind _returnvalue_2 (Math|Float|Truncate _returnvalue))
  (bind _returnvalue_3 (Spline|GetDistanceAlongSplineatSplinePoint InputPin _returnvalue_2))
  (return (+ (* (- (Spline|GetDistanceAlongSplineatSplinePoint InputPin (Math|Float|Truncate (+ _returnvalue 1.0))) _returnvalue_3) (- _returnvalue (Math|Conversions|ToFloat(Integer) _returnvalue_2))) _returnvalue_3) 0))

(fn AdaptiveTextureTexture
  (params (InputPin :type Material%20Instance%20Dynamic%20Object%20Reference) (Value :type Texture%202D%20Object%20Reference))
  (bind _returnvalue (Class|Texture2D|BlueprintGetSizeY Value))
  (bind _returnvalue_2 (Class|Texture2D|BlueprintGetSizeX Value))
  (bind _returnvalue_3 (Math|Conversions|ToFloat(Integer) _returnvalue_2))
  (bind _returnvalue_4 (Math|Conversions|ToFloat(Integer) _returnvalue))
  (Rendering|Material|SetTextureParameterValue InputPin "Texture" Value)
  (if (> _returnvalue_2 _returnvalue)
    (Rendering|Material|SetScalarParameterValue InputPin "Y" (/ _returnvalue_4 _returnvalue_3) :!class /Script/Engine.MaterialInstanceDynamic)
    (Rendering|Material|SetScalarParameterValue InputPin "X" 1.0 :!class /Script/Engine.MaterialInstanceDynamic)
    (else
      (Rendering|Material|SetScalarParameterValue InputPin "X" (/ _returnvalue_3 _returnvalue_4) :!class /Script/Engine.MaterialInstanceDynamic)
      (Rendering|Material|SetScalarParameterValue InputPin "Y" 1.0 :!class /Script/Engine.MaterialInstanceDynamic))))