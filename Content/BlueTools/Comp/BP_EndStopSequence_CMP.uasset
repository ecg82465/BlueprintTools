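; Actor component for a Level Sequence Actor that pauses its sequence just before playback reaches the end.
; Every Tick it casts its owner to LevelSequenceActor and, while the player is playing, compares playback position to playback end.
; Once the remaining playback is within a small fixed threshold, it calls Pause, so the sequence stops short of finishing.
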(event EventBeginPlay)

(event EventTick
  (params (DeltaSeconds :type Float%20%28single-precision%29))
  (bind _aslevel_sequence_actor (Utilities|Casting|CastToLevelSequenceActor (Components|GetOwner)))
  (if (and (Audio|Components|Audio|IsPlaying (Variables|/Script/LevelSequence.LevelSequenceActor|GetSequencePlayer _aslevel_sequence_actor)) (<= (- (Class|MovieSceneSequencePlayer|GetPlaybackEnd (Variables|/Script/LevelSequence.LevelSequenceActor|GetSequencePlayer _aslevel_sequence_actor)) (Components|Timeline|GetPlaybackPosition (Variables|/Script/LevelSequence.LevelSequenceActor|GetSequencePlayer _aslevel_sequence_actor))) 0.1))
    (Sequencer|Player|Pause (Variables|/Script/LevelSequence.LevelSequenceActor|GetSequencePlayer _aslevel_sequence_actor))))